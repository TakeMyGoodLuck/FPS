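; Inventory item Blueprint for drinking water that restores the player's thirst when its skill is used.
; ItemSkill casts player zero's character to FirstPersonCharacter and calls DoSatisfyThirts on its HungerAndThirstStats with a fixed amount.
; All other events are disabled stubs, and the construction script only calls its parent.
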(event EventBeginPlay
  (|CallParentFunction) ; This node is disabled and will not be called.\nDrag off pins to build functionality.
)

(event Collision|EventActorBeginOverlap
  (params (OtherActor :type Actor%20Object%20Reference))
  (|CallParentFunction OtherActor) ; This node is disabled and will not be called.\nDrag off pins to build functionality.
)

(event EventTick
  (params (DeltaSeconds :type Float%20%28single-precision%29))
  (|CallParentFunction DeltaSeconds) ; This node is disabled and will not be called.\nDrag off pins to build functionality.
)

(event EventItemSkill
  (bind _asfirst_person_character (Utilities|Casting|CastToFirstPersonCharacter (Game|GetPlayerCharacter 0)))
  (Default|DoSatisfyThirts (Variables|/Game/FirstPersonBP/Blueprints/FirstPersonCharacter.FirstPersonCharacter_C|GetHunger_and_Thirst_Stats _asfirst_person_character) 25.0))

(fn ConstructionScript
  (|CallParentFunction))