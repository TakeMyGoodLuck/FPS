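; BP_WorldActor is a world item actor that represents an inventory item placed in the level.
; On BeginPlay it sets its static mesh from the class defaults of its assigned Item class.
; It also passes that item's name, stackable flag and the actor's Amount to a WorldItemWB widget component to label the item.
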(event EventBeginPlay
  ;[1 1 1] Устанавливаем 3d mesh и название предмета
  (CallFunction|Initialize3dMesh)
  (CallFunction|InitializeItemName))

(fn ConstructionScript)

(fn Initialize3dMesh
  (Components|StaticMesh|SetStaticMesh (Variables|Default|GetItemMesh) (.3dmesh (Utilities|GetClassDefaults (Variables|Default|GetItem)))))

(fn InitializeItemName
  (bind _item (Variables|Default|GetItem))
  (bind _itemsignature (Utilities|GetClassDefaults _item))
  (bind _asworld_item_wb (Utilities|Casting|CastToWorldItemWB (UserInterface|GetUserWidgetObject (Variables|Default|GetWidget))))
  (Default|SetItemName _asworld_item_wb (.name _itemsignature) (.stackablecanbestacked _itemsignature) (Variables|Default|GetAmount)))