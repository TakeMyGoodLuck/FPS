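; BFL is a Blueprint function library of shortcut getters for common gameplay objects.
; It casts player 0's character to BP_TestPlayer and exposes that character's ACBasePlayerStats through a second getter built on the first.
; A separate getter returns the game instance cast to BP_GameInstance.
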(fn GetTestCharacter
  (bind _asbp_test_player (Utilities|Casting|CastToBP_TestPlayer (Game|GetPlayerCharacter 0)))
  (return _asbp_test_player))

(fn GetPlayerStats
  (return (Variables|/Game/BP_TestPlayer.BP_TestPlayer_C|GetAC_BasePlayerStats (CallFunction|GetTestCharacter))))

(fn GetGI
  (bind _asbp_game_instance (Utilities|Casting|CastToBP_GameInstance (Game|GetGameInstance)))
  (return _asbp_game_instance))