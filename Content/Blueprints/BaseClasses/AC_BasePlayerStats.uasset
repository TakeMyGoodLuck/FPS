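; Player stats component that presents survival stats (stamina, energy, hunger, thirst, temperature) and sleep sequences to the player.
; On BeginPlay it creates the stats HUD and caches its widgets, which the stat events update.
; Hunger or thirst wake events show a disturbance widget.
; Sleep and overheat events toggle input and fade the camera, adding a bed view blend or character overheat state; sleep end and zero temperature also update quests.
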(event EventBeginPlay
  (bind _returnvalue (Actor|GetActorOfClass "/Script/FPS.CoreWorldTimeManager"))
  (Variables|Default|SetTimeManager _returnvalue)
  (bind _returnvalue_2 (UserInterface|CreateWidget "/Game/Blueprints/WidgetBlueprints/PlayerStats/WBP_StatsHud.WBP_StatsHud_C"))
  (bind _output_get (Variables|Default|SetStatsHud _returnvalue_2))
  (UserInterface|Viewport|AddtoViewport _output_get 0)
  (Variables|Default|SetWBP%20Stamina (Variables|/Game/Blueprints/WidgetBlueprints/PlayerStats/WBP_StatsHud.WBP_StatsHud_C|GetWBP_Stamina (Variables|Default|GetStatsHud)))
  (Variables|Default|SetWBP%20Energy (Variables|/Game/Blueprints/WidgetBlueprints/PlayerStats/WBP_StatsHud.WBP_StatsHud_C|GetWBP_Energy (Variables|Default|GetStatsHud)))
  (Variables|Default|SetWBP%20Hungry (Variables|/Game/Blueprints/WidgetBlueprints/PlayerStats/WBP_StatsHud.WBP_StatsHud_C|GetWBP_Hungry (Variables|Default|GetStatsHud)))
  (Variables|Default|SetWBP%20Thirst (Variables|/Game/Blueprints/WidgetBlueprints/PlayerStats/WBP_StatsHud.WBP_StatsHud_C|GetWBP_Thirst (Variables|Default|GetStatsHud)))
  (Variables|Default|SetWBP%20Temperature (Variables|/Game/Blueprints/WidgetBlueprints/PlayerStats/WBP_StatsHud.WBP_StatsHud_C|GetWBP_Temperature (Variables|Default|GetStatsHud))))

(event EventOnHungry
  (params (Hungry :type Float%20%28single-precision%29))
  (Default|SetHungry (Variables|Default|GetWBP%20Hungry) Hungry)
  (Development|PrintString "Hello"))

(event EventOnSleepStarted
  (Input|DisableInput (Game|GetPlayerCharacter 0) (Game|GetPlayerController 0))
  (bind _returnvalue (Actor|GetActorOfClass "/Game/Blueprints/BaseClasses/BP_BaseBed.BP_BaseBed_C"))
  (Game|Player|SetViewTargetwithBlend (Game|GetPlayerController 0) _returnvalue 0.75 "VTBlend_Linear" 0.0 false)
  (Utilities|FlowControl|Delay 0.75)
  (CameraFades|StartCameraFade (Game|GetPlayerCameraManager 0) 0.0 0.99 1.0 "(R=0.000200,G=0.000000,B=0.005000,A=1.000000)" false true)
  (Utilities|FlowControl|Delay 0.5)
  (bind _returnvalue_2 (Audio|SpawnSound2D "/Game/Sounds/Object/S_Bed.S_Bed" 1.0 1.0 0.0 0))
  (Audio|Components|Audio|StopDelayed _returnvalue_2 3.75))

(event EventOnOverheatSleepEnded
  (bind _testcharacter (CallFunction|GetTestCharacter))
  (CameraFades|StartCameraFade (Game|GetPlayerCameraManager 0) 0.99 0.0 1.0 "(R=0.000200,G=0.000000,B=0.005000,A=1.000000)" false true)
  (Input|EnableInput (Game|GetPlayerCharacter 0) (Game|GetPlayerController 0))
  (Default|Overheat _testcharacter false)
  (Utilities|FlowControl|Delay 1.0)
  (Variables|/Script/Engine.CameraComponent|SetbUsePawnControlRotation (Variables|/Game/BP_TestPlayer.BP_TestPlayer_C|GetCamera _testcharacter) true))

(event EventOnOverheatSleepStarted
  (Input|DisableInput (Game|GetPlayerCharacter 0) (Game|GetPlayerController 0))
  (CameraFades|StartCameraFade (Game|GetPlayerCameraManager 0) 0.0 0.99 1.0 "(R=0.000200,G=0.000000,B=0.005000,A=1.000000)" false true)
  (Variables|/Script/Engine.CameraComponent|SetbUsePawnControlRotation (Variables|/Game/BP_TestPlayer.BP_TestPlayer_C|GetCamera (CallFunction|GetTestCharacter)) false)
  (Default|Overheat (CallFunction|GetTestCharacter) true))

(event EventOnStaminaReduced
  (params (Stamina :type Float%20%28single-precision%29))
  (Default|SetStamina (Variables|Default|GetWBP%20Stamina) Stamina))

(event EventOnStaminaRestoring
  (params (Stamina :type Float%20%28single-precision%29))
  (Default|RestoreStamina (Variables|Default|GetWBP%20Stamina) Stamina))

(event EventWakeonHunger
  (bind _returnvalue (UserInterface|CreateWidget "/Game/Blueprints/WidgetBlueprints/PlayerStats/WBP_SleepDisturb.WBP_SleepDisturb_C" 0 "Hunger"))
  (UserInterface|Viewport|AddtoViewport _returnvalue 0))

(event EventOnThirst
  (params (Thirst :type Float%20%28single-precision%29))
  (Default|SetThirst (Variables|Default|GetWBP%20Thirst) Thirst))

(event EventOnEnergy
  (params (Energy :type Float%20%28single-precision%29))
  (Default|SetEnergy (Variables|Default|GetWBP%20Energy) Energy))

(event EventWakeonThirst
  (bind _returnvalue (UserInterface|CreateWidget "/Game/Blueprints/WidgetBlueprints/PlayerStats/WBP_SleepDisturb.WBP_SleepDisturb_C" 0 "Thirst"))
  (UserInterface|Viewport|AddtoViewport _returnvalue 0))

(event EventOnTemperatureUpdated
  (params (Temperature :type Float%20%28single-precision%29))
  (bind _returnvalue (Subsystems|GetCoreQuestSubsystem))
  (Default|UpdateTemperature (Variables|Default|GetWBP%20Temperature) Temperature)
  (if (== Temperature 0.0)
    (Class|CoreQuestSubsystem|UpdateQuest _returnvalue (Class|CoreQuestSubsystem|GetQuestHolder _returnvalue) 1)))

(event EventOnSleepEnded
  (bind _returnvalue (Game|GetPlayerCharacter 0))
  (bind _returnvalue_2 (Game|GetPlayerController 0))
  (bind _returnvalue_3 (Subsystems|GetCoreQuestSubsystem))
  (CameraFades|StartCameraFade (Game|GetPlayerCameraManager 0) 0.99 0.0 1.0 "(R=0.000200,G=0.000000,B=0.005000,A=1.000000)" false true)
  (Utilities|FlowControl|Delay 1.0)
  (Game|Player|SetViewTargetwithBlend _returnvalue_2 _returnvalue 0.5 "VTBlend_Linear" 0.0 false)
  (Input|EnableInput _returnvalue _returnvalue_2)
  (Class|CoreQuestSubsystem|UpdateQuest _returnvalue_3 (Class|CoreQuestSubsystem|GetQuestHolder _returnvalue_3)))