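; Farmable ground tile that spawns grass on BeginPlay and moves through Grassed, Weeded, Plowed and Seeded states as tools are used.
; InteractCheck validates tool against state, while InstrumentUsed swaps the attached grass or plant, changes the plane material, plays sounds and updates quest zones and the quest subsystem.
; Interactt combines check and action, also forwarding Scythe and Gloves to the attached actor.
; Outline toggles custom depth and the use hint.
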(event EventBeginPlay
  (bind _returnvalue (Game|SpawnActorfromClass "/Game/Blueprints/GameplayObjects/BP_Grass.BP_Grass_C" (Math|Transform|MakeTransform "0, 0, 0" "0, 0, 0" "1,1,1") "Undefined" 0 0))
  (bind _output_get (Variables|Default|SetNewVar_0 _returnvalue))
  (Transformation|AttachActorToActor _output_get self "None" "KeepRelative" "KeepRelative" "KeepRelative" true)
  (bind _asbp_base_grass (Utilities|Casting|CastToBP_BaseGrass (Variables|Default|GetNewVar_0)))
  (Collision|SetCollisionResponsetoChannel (Variables|/Game/Blueprints/BaseClasses/BP_BaseGrass.BP_BaseGrass_C|GetBox _asbp_base_grass) "ECC_GameTraceChannel4" "ECR_Block")
  (Variables|Default|SetGroundType "Grassed"))

(event Collision|EventActorBeginOverlap
  (params (OtherActor :type Actor%20Object%20Reference)))

(event EventTick
  (params (DeltaSeconds :type Float%20%28single-precision%29)))

(event EventOutline
  (params (Start :type Boolean) (Tool :type Core%20Instrument%20Object%20Object%20Reference))
  (bind _game_instance (CallFunction|GetGI))
  (bind _plane (Variables|Default|GetPlane))
  (bind _usekey (Variables|Default|GetUseKey))
  (bind _usetext (Variables|Default|GetUseText))
  (Utilities|IsValid Tool
    (:Is%20Valid
      (Rendering|SetRenderCustomDepth _plane Start)
      (Default|ShowUseHint _game_instance _usekey _usetext Start)
      (bind _newvar_0 (Variables|Default|GetNewVar_0)
        (:then)
        (:else)))
    (:Is%20Not%20Valid
      (Rendering|SetRenderCustomDepth _plane false)
      (Default|ShowUseHint _game_instance _usekey _usetext false)
      (bind _newvar_0_2 (Variables|Default|GetNewVar_0)
        (:then)
        (:else)))))

(event EventInstrumentUsed
  (params (Instrument :type Core%20Instrument%20Object%20Object%20Reference))
  (bind _instrtype (Variables|/Script/FPS.CoreInstrumentObject_|GetInstrType Instrument))
  (bind _returnvalue (Utilities|Select :Index _instrtype :Scythe 0 :Hoe 1 :Rake 2 :Seeds 3 :Bucket 4 :Gloves 5 :Hammer 6))
  (switch Utilities|FlowControl|Switch|SwitchonEInstrumentType _instrtype
    (:Hoe
      (bind _newvar_0 (Variables|Default|GetNewVar_0)
        (:then
          (Actor|DestroyActor _newvar_0)
          (Variables|Default|SetGroundType "Weeded")
          (Variables|Default|SetNewVar_0 0))
        (:else)))
    (:Rake
      (Rendering|Material|SetMaterial (Variables|Default|GetPlane) 0 "/Game/wildtextures_plowed-field-4k-seamless-texture_Mat_Inst.wildtextures_plowed-field-4k-seamless-texture_Mat_Inst")
      (Variables|Default|SetGroundType "Plowed"))
    (:Seeds
      (bind _returnvalue_2 (Game|SpawnActorfromClass "/Game/Blueprints/GameplayObjects/BP_Plant.BP_Plant_C" (Math|Transform|MakeTransform "-7.000000,15.000000, 0" "0, 0, 0" "1,1,1") "Undefined" 0 self 0))
      (bind _output_get (Variables|Default|SetNewVar_0 _returnvalue_2))
      (Transformation|AttachActorToActor _output_get self "None" "KeepRelative" "KeepRelative" "KeepRelative" true)
      (Variables|Default|SetGroundType "Seeded"))
    (:Bucket
      (Rendering|Material|SetScalarParameterValueonMaterials (Variables|Default|GetPlane) "Param" 0.5)))
  (Audio|SpawnSoundAttached (Utilities|Select :Index _instrtype :Scythe 0 :Hoe "/Game/Sounds/Tools/S_Hoe.S_Hoe" :Rake "/Game/Sounds/Tools/S_Rake.S_Rake" :Seeds "/Game/Sounds/Tools/S_Seeds.S_Seeds" :Bucket "/Game/Sounds/Tools/S_Bucket.S_Bucket" :Gloves 0 :Hammer 0) (Variables|Default|GetPlane) "None" "0, 0, 0" "0, 0, 0" "KeepRelativeOffset" false 1.0 1.0 0.0 "/Game/Sounds/NewSoundAttenuation.NewSoundAttenuation" 0)
  (for _array_element (Collision|GetOverlappingActors (Variables|Default|GetBox) "/Game/Blueprints/BaseClasses/BP_QuestZOne.BP_QuestZOne_C" :!class /Script/Engine.PrimitiveComponent)
    (bind _asbp_quest_zone (Utilities|Casting|CastToBP_QuestZOne _array_element))
    (Default|UpdateQuest _asbp_quest_zone self _returnvalue))
  (Class|CoreQuestSubsystem|UpdateQuest (Subsystems|GetCoreQuestSubsystem) self _returnvalue))

(fn ConstructionScript)

(fn InteractCheck
  (params (Instrument :type Core%20Instrument%20Object%20Object%20Reference))
  (bind _groundtype (Variables|Default|GetGroundType))
  (bind _output_get (Variables|Default|SetLocalTool Instrument))
  (switch Utilities|FlowControl|Switch|SwitchonEInstrumentType (Variables|/Script/FPS.CoreInstrumentObject_|GetInstrType _output_get)
    (:Hoe
      (bind _ascore_grass_actor (Utilities|Casting|CastToCoreGrassActor (Variables|Default|GetNewVar_0))
        (:then
          (if (< (Class|CoreGrassActor|GetState _ascore_grass_actor) 2)
            (bind _newvar_0 (Variables|Default|GetNewVar_0)
              (:then
                (return true))
              (:else
                _))
            (else
              (Development|PrintString "Grass is too high")))
          (return false))
        (:CastFailed
          (return false))))
    (:Rake
      (if (Utilities|Enum|Equal(Enum) _groundtype "Weeded")
        (return true)
        (else
          _)))
    (:Seeds
      (Variables|Default|GetNewVar_0
        (:then)
        (:else
          (if (Utilities|Enum|Equal(Enum) _groundtype "Plowed")
            (return true)
            (else
              _)))))
    (:Bucket
      (Variables|Default|GetNewVar_0
        (:then
          (if (Utilities|Enum|Equal(Enum) (Variables|Default|GetGroundType) "Seeded")
            (return true)
            (else
              (return false))))
        (:else
          (return false))))
    (:Gloves
      (Variables|Default|GetNewVar_0
        (:then
          (if (Utilities|Enum|Equal(Enum) (Variables|Default|GetGroundType) "Seeded")
            _
            (else
              _)))
        (:else
          _))
      (return false))
    (:Hammer
      (return false)))
  (return false))

(fn Interactt
  (params (Tool :type Core%20Instrument%20Object%20Object%20Reference))
  (LocalVariables|SetLocalTool Tool)
  (switch Utilities|FlowControl|Switch|SwitchonEInstrumentType (Variables|/Script/FPS.CoreInstrumentObject_|GetInstrType Tool)
    (:Scythe
      (bind _interacted_ (Class|BPIInteraction|Interactt(Message) (Variables|Default|GetNewVar_0) (LocalVariables|GetLocalTool)))
      (return _interacted_))
    (:Hoe
      (bind _asbp_base_grass (Utilities|Casting|CastToBP_BaseGrass (Variables|Default|GetNewVar_0))
        (:then
          (if (< (Class|CoreGrassActor|GetState _asbp_base_grass) 2)
            (bind _newvar_0 (Variables|Default|GetNewVar_0)
              (:then
                (Actor|DestroyActor _newvar_0)
                (Variables|Default|SetGroundType "Weeded")
                (Variables|Default|SetNewVar_0 0)
                (return true))
              (:else
                (return false)))
            (else
              (Development|PrintString "Grass is too high")
              (return false))))
        (:CastFailed
          (return false))))
    (:Rake
      (if (Utilities|Enum|Equal(Enum) (Variables|Default|GetGroundType) "Weeded")
        (Rendering|Material|SetMaterial (Variables|Default|GetPlane) 0 "/Game/wildtextures_plowed-field-4k-seamless-texture_Mat_Inst.wildtextures_plowed-field-4k-seamless-texture_Mat_Inst")
        (Variables|Default|SetGroundType "Plowed")
        (return true)
        (else
          (return false))))
    (:Seeds
      (Variables|Default|GetNewVar_0
        (:then
          (return false))
        (:else
          (if (Utilities|Enum|Equal(Enum) (Variables|Default|GetGroundType) "Plowed")
            (bind _returnvalue (Game|SpawnActorfromClass "/Game/Blueprints/GameplayObjects/BP_Plant.BP_Plant_C" (Math|Transform|MakeTransform "-7.000000,15.000000, 0" "0, 0, 0" "1,1,1") "Undefined" 0 0 0))
            (bind _output_get (Variables|Default|SetNewVar_0 _returnvalue))
            (Transformation|AttachActorToActor _output_get self "None" "KeepRelative" "KeepRelative" "KeepRelative" true)
            (Variables|Default|SetGroundType "Seeded")
            (return true)
            (else
              (return false))))))
    (:Bucket
      (Variables|Default|GetNewVar_0
        (:then
          (if (Utilities|Enum|Equal(Enum) (Variables|Default|GetGroundType) "Seeded")
            (Rendering|Material|SetScalarParameterValueonMaterials (Variables|Default|GetPlane) "Param" 0.5)
            (return true)
            (else
              (return false))))
        (:else
          (return false))))
    (:Gloves
      (Variables|Default|GetNewVar_0
        (:then
          (if (Utilities|Enum|Equal(Enum) (Variables|Default|GetGroundType) "Seeded")
            (bind _interacted__2 (Class|BPIInteraction|Interactt(Message) (Variables|Default|GetNewVar_0) (LocalVariables|GetLocalTool)))
            (if _interacted__2
              (Actor|DestroyActor (Variables|Default|GetNewVar_0))
              (Variables|Default|SetNewVar_0 0)
              (Variables|Default|SetGroundType "Plowed")
              (return true)
              (else
                (return false)))
            (else
              (return false))))
        (:else
          (return false))))))