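; BP_WaterFilling is an interactable water source, apparently a well, where the player fills a bucket tool.
; Interacting with a bucket below capacity fills it, drains player stamina and energy, updates the quest subsystem and plays the well sound.
; The Outline event toggles a custom-depth highlight and interact hint, showing them only for bucket tools.
; The InteractCheck and Interactt functions are stubs that return false.
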(event EventBeginPlay)

(event Collision|EventActorBeginOverlap
  (params (OtherActor :type Actor%20Object%20Reference)))

(event EventTick
  (params (DeltaSeconds :type Float%20%28single-precision%29)))

(event EventOutline
  (params (Start :type Boolean) (Tool :type Core%20Instrument%20Object%20Object%20Reference))
  (bind _game_instance (CallFunction|GetGI))
  (bind _interactkey (Variables|Default|GetInteractKey))
  (bind _interacttext (Variables|Default|GetInteractText))
  (bind _visualmesh (Variables|Default|GetVisualMesh))
  (Utilities|Casting|CastToB_BaseBucketObject Tool
    (:then
      (Rendering|SetRenderCustomDepth _visualmesh Start)
      (Default|ShowInteractHint _game_instance _interactkey _interacttext Start))
    (:CastFailed
      (Rendering|SetRenderCustomDepth _visualmesh false)
      (Default|ShowInteractHint _game_instance _interactkey _interacttext false))))

(event EventInteracted
  (params (Instrument :type Core%20Instrument%20Object%20Object%20Reference))
  (bind _player_stats (CallFunction|GetPlayerStats))
  (bind _asb_base_bucket_object (Utilities|Casting|CastToB_BaseBucketObject Instrument))
  (if (< (Variables|/Script/FPS.CoreActionInstruments|Getfilling _asb_base_bucket_object) (Variables|/Script/FPS.CoreActionInstruments|Getcapacity _asb_base_bucket_object))
    (Class|CoreActionInstruments|Fill _asb_base_bucket_object)
    (Class|CorePlayerStats|StaminaReduce _player_stats (Variables|Default|GetStamina%20Consume))
    (Class|CorePlayerStats|ReduceEnergy _player_stats (Variables|Default|GetEnergy%20Consume))
    (Class|CoreQuestSubsystem|UpdateQuest (Subsystems|GetCoreQuestSubsystem) self)
    (Audio|SpawnSoundAttached "/Game/Sounds/Object/S_Well.S_Well" (Variables|Default|GetVisualMesh) "None" "0, 0, 0" "0, 0, 0" "KeepRelativeOffset" false 1.0 1.0 0.0 0 0)))

(fn ConstructionScript)

(fn InteractCheck
  (params (Instrument :type Core%20Instrument%20Object%20Object%20Reference))
  (return false))

(fn Interactt
  (params (Tool :type Core%20Instrument%20Object%20Object%20Reference))
  (return false))