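; BP_BaseWorkbench is a base workbench actor where damaged tools are repaired.
; Outline toggles custom depth on the visual mesh while a valid tool is supplied.
; Interacted casts the instrument to CoreToolObject and, below full health, repairs it, charges stamina and energy, and updates quests by instrument type.
; InteractCheck always returns false and Interactt is empty.
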(event EventBeginPlay)

(event Collision|EventActorBeginOverlap
  (params (OtherActor :type Actor%20Object%20Reference)))

(event EventTick
  (params (DeltaSeconds :type Float%20%28single-precision%29)))

(event EventOutline
  (params (Start :type Boolean) (Tool :type Core%20Instrument%20Object%20Object%20Reference))
  (bind _visualmesh (Variables|Default|GetVisualMesh))
  (Utilities|IsValid Tool
    (:Is%20Valid
      (Rendering|SetRenderCustomDepth _visualmesh Start))
    (:Is%20Not%20Valid
      (Rendering|SetRenderCustomDepth _visualmesh false))))

(event EventInteracted
  (params (Instrument :type Core%20Instrument%20Object%20Object%20Reference))
  (bind _player_stats (CallFunction|GetPlayerStats))
  (bind _ascore_tool_object (Utilities|Casting|CastToCoreToolObject Instrument))
  (if (< (Class|CoreToolObject|GetHealth _ascore_tool_object) 1e+02)
    (Class|CoreToolObject|RepairTool _ascore_tool_object)
    (Class|CorePlayerStats|StaminaReduce _player_stats (Variables|Default|GetStamina%20Cost))
    (Class|CorePlayerStats|ReduceEnergy _player_stats (Variables|Default|GetEnergy%20Cost))
    (Class|CoreQuestSubsystem|UpdateQuest (Subsystems|GetCoreQuestSubsystem) self (Utilities|Select :Index (Variables|/Script/FPS.CoreInstrumentObject_|GetInstrType Instrument) :Scythe 0 :Hoe 1 :Rake 2 :Seeds 3 :Bucket 4 :Gloves 5 :Hammer 6))))

(fn ConstructionScript)

(fn InteractCheck
  (params (Instrument :type Core%20Instrument%20Object%20Object%20Reference))
  (return false))

(fn Interactt
  (params (Tool :type Core%20Instrument%20Object%20Object%20Reference)))