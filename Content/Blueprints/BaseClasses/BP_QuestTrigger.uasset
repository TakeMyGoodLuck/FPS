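; BP_QuestTrigger is a base trigger actor that reports quest interactions when something begins overlapping its Box component.
; On overlap, it passes itself and its InteractType to UpdateQuest on every BP_QuestZOne actor overlapping the box, printing a debug string for each.
; It then sends the same update to the CoreQuestSubsystem, with no check on which actor triggered the overlap.
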(event OnComponentBeginOverlap(Box)
  (params (OverlappedComponent :type Primitive%20Component%20Object%20Reference) (OtherActor :type Actor%20Object%20Reference) (OtherComp :type Primitive%20Component%20Object%20Reference) (OtherBodyIndex :type Integer) (bFromSweep :type Boolean) (SweepResult :type Hit%20Result%20Structure%20%28by%20ref%29))
  (bind _interact_type (Variables|Quest|GetInteract%20Type))
  (for _array_element (Collision|GetOverlappingActors (Variables|Default|GetBox) "/Game/Blueprints/BaseClasses/BP_QuestZOne.BP_QuestZOne_C" :!class /Script/Engine.PrimitiveComponent)
    (bind _asbp_quest_zone (Utilities|Casting|CastToBP_QuestZOne _array_element))
    (Default|UpdateQuest _asbp_quest_zone self _interact_type)
    (Development|PrintString "1"))
  (Class|CoreQuestSubsystem|UpdateQuest (Subsystems|GetCoreQuestSubsystem) self _interact_type))

(event EventBeginPlay)

(event Collision|EventActorBeginOverlap
  (params (OtherActor :type Actor%20Object%20Reference)))

(event EventTick
  (params (DeltaSeconds :type Float%20%28single-precision%29)))

(fn ConstructionScript)