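; BP_BaseBed is a base bed Blueprint that can be outlined, with interaction stubbed out.
; The Outline event toggles custom depth rendering on its static mesh.
; Interact and Interactt both just return false.
; A disconnected chain in Interact would call Sleep on the BP_TestPlayer's ACBasePlayerStats component and print a debug string, but it never runs.
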(event EventBeginPlay)

(event Collision|EventActorBeginOverlap
  (params (OtherActor :type Actor%20Object%20Reference)))

(event EventTick
  (params (DeltaSeconds :type Float%20%28single-precision%29)))

(event EventOutline
  (params (Start :type Boolean) (Tool :type Core%20Instrument%20Object%20Object%20Reference))
  (Rendering|SetRenderCustomDepth (Variables|Default|GetStaticMeshComponent) Start))

(fn ConstructionScript)

(fn Interact
  (params (Instrument :type Core%20Instrument%20Object%20Object%20Reference))
  (return false))

(fn Interactt
  (params (Tool :type Core%20Instrument%20Object%20Object%20Reference))
  (return false))