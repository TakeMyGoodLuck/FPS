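; Base trash actor that the player can remove only with gloves.
; Outline toggles custom depth on the visual mesh when the tool is a gloves object.
; Interact requires a Gloves instrument and quest subsystem approval, then destroys the actor and updates the quest.
; A separate Interactt function checks the tool class and destroys the actor without involving quests.
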(event EventBeginPlay)

(event Collision|EventActorBeginOverlap
  (params (OtherActor :type Actor%20Object%20Reference)))

(event EventTick
  (params (DeltaSeconds :type Float%20%28single-precision%29)))

(event EventOutline
  (params (Start :type Boolean) (Tool :type Core%20Instrument%20Object%20Object%20Reference))
  (bind _visualmesh (Variables|Default|GetVisualMesh))
  (if (Utilities|ClassIsChildOf (Utilities|GetClass Tool) "/Script/FPS.CoreGlovesObject")
    (Rendering|SetRenderCustomDepth _visualmesh Start)
    (else
      (Rendering|SetRenderCustomDepth _visualmesh false))))

(fn ConstructionScript)

(fn Interact
  (params (Instrument :type Core%20Instrument%20Object%20Object%20Reference))
  (if (Utilities|Enum|Equal(Enum) (Variables|/Script/FPS.CoreInstrumentObject_|GetInstrType Instrument) "Gloves")
    (bind _result (Class|CoreQuestSubsystem|CheckQuestActor (Subsystems|GetCoreQuestSubsystem) self))
    (if _result
      (Actor|DestroyActor)
      (Class|CoreQuestSubsystem|UpdateQuest (Subsystems|GetCoreQuestSubsystem) self)
      (return true))
    (else
      (return false))))

(fn Interactt
  (params (Tool :type Core%20Instrument%20Object%20Object%20Reference))
  (if (Utilities|ClassIsChildOf (Utilities|GetClass Tool) "/Script/FPS.CoreGlovesObject")
    (Actor|DestroyActor)
    (return true)
    (else
      (return false))))