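; Base plant Blueprint that grows in timed stages and can be harvested with gloves once at its maximum state.
; After a random start delay, a timer at the plant's growth speed calls GrowPlant, and each growth event rescales the mesh height and restarts the timer.
; Gloves enable the custom-depth outline and pass the interaction checks at full growth, and interacting shows a harvest count popup widget.
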(event Custom|Set%20Timer
  (bind _returnvalue (Utilities|Time|SetTimerbyEvent (delegate Custom|CustomEvent_0) (Class|CorePlantA|GetSpd)))
  (Variables|Default|SetTimer _returnvalue))

(event Custom|CustomEvent_0
  (Class|CorePlantA|GrowPlant))

(event EventBeginPlay
  (Transformation|SetRelativeScale3D (Variables|Default|GetVisualMesh) (Math|Vector|MakeVector 1.0 1.0 0.1))
  (Utilities|FlowControl|Delay (Math|Random|RandomFloatinRange 0.0 5.0))
  (CallFunction|SetTimer))

(event Collision|EventActorBeginOverlap
  (params (OtherActor :type Actor%20Object%20Reference)))

(event EventTick
  (params (DeltaSeconds :type Float%20%28single-precision%29)))

(event EventOnPlantGrowed
  (params (Growth_State :type Integer))
  (Transformation|SetRelativeScale3D (Variables|Default|GetVisualMesh) (Math|Vector|MakeVector 1.0 1.0 (Utilities|Select :Index Growth_State :Option%200 0.1 :Option%201 0.25 :Option%202 0.5 :Option%203 1.0)))
  (CallFunction|SetTimer))

(event EventOutline
  (params (Start :type Boolean) (Tool :type Core%20Instrument%20Object%20Object%20Reference))
  (bind _visualmesh (Variables|Default|GetVisualMesh))
  (if (Utilities|ClassIsChildOf (Utilities|GetClass Tool) "/Script/FPS.CoreGlovesObject")
    (Rendering|SetRenderCustomDepth _visualmesh Start)
    (else
      (Rendering|SetRenderCustomDepth _visualmesh false))))

(event EventInteract
  (params (Instrument :type Core%20Instrument%20Object%20Object%20Reference))
  (bind _returnvalue (UserInterface|CreateWidget "/Game/Blueprints/WidgetBlueprints/WBP_CountText.WBP_CountText_C" 0 (Utilities|Text|ToText(String) (Utilities|String|Append "+" (Utilities|String|ToString(Integer) (Variables|Default|GetHarvestPerSeed)) " " (Utilities|String|ToString(Name) (Variables|Default|GetName))))))
  (UserInterface|Viewport|AddtoViewport _returnvalue 0))

(fn ConstructionScript)

(fn InteractCheck
  (params (Instrument :type Core%20Instrument%20Object%20Object%20Reference))
  (if (Utilities|Enum|Equal(Enum) (Variables|/Script/FPS.CoreInstrumentObject_|GetInstrType Instrument) "Gloves")
    (if (== (Class|CorePlantA|GetState) (Variables|Default|GetMaxStates))
      (return true)
      (else
        (return false)))
    (else
      (return false))))

(fn Interactt
  (params (Tool :type Core%20Instrument%20Object%20Object%20Reference))
  (if (Utilities|ClassIsChildOf (Utilities|GetClass Tool) "/Script/FPS.CoreGlovesObject")
    (if (== (Class|CorePlantA|GetState) (Variables|Default|GetMaxStates))
      (bind _returnvalue (UserInterface|CreateWidget "/Game/Blueprints/WidgetBlueprints/WBP_CountText.WBP_CountText_C" 0 (Utilities|Text|ToText(String) (Utilities|String|Append "+" (Utilities|String|ToString(Integer) (Variables|Default|GetHarvestPerSeed)) " " (Utilities|String|ToString(Name) (Variables|Default|GetName))))))
      (UserInterface|Viewport|AddtoViewport _returnvalue 0)
      (return true)
      (else
        (return false)))
    (else
      (return false))))