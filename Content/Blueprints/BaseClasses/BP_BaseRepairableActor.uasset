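; Base repairable actor that starts with a broken mesh and can be fixed with a hammer to advance quests.
; Outline shows custom-depth highlighting and a use hint only for a hammer tool while the actor is broken, and InteractCheck applies the same condition.
; InstrumentUsed swaps in the repaired mesh, clears the broken flag, plays a random hammer sound, then updates overlapping quest zones and the core quest subsystem.
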(event EventBeginPlay)

(event Collision|EventActorBeginOverlap
  (params (OtherActor :type Actor%20Object%20Reference)))

(event EventTick
  (params (DeltaSeconds :type Float%20%28single-precision%29)))

(event EventOutline
  (params (Start :type Boolean) (Tool :type Core%20Instrument%20Object%20Object%20Reference))
  (bind _game_instance (CallFunction|GetGI))
  (bind _visualmesh (Variables|Default|GetVisualMesh))
  (bind _usekey (Variables|Default|GetUseKey))
  (bind _usetext (Variables|Default|GetUseText))
  (if (and (Utilities|ClassIsChildOf (Utilities|GetClass Tool) "/Game/Blueprints/BaseClasses/InstrumentObjects/BP_BaseHammerObject.BP_BaseHammerObject_C") (Variables|Default|GetIsBroken))
    (Rendering|SetRenderCustomDepth _visualmesh Start)
    (Default|ShowUseHint _game_instance _usekey _usetext Start)
    (else
      (Rendering|SetRenderCustomDepth _visualmesh false)
      (Default|ShowUseHint _game_instance _usekey _usetext false))))

(event EventInstrumentUsed
  (params (Instrument :type Core%20Instrument%20Object%20Object%20Reference))
  (bind _self self)
  (Components|StaticMesh|SetStaticMesh (Variables|Default|GetVisualMesh) (Variables|Default|GetRMesh))
  (Variables|Default|SetIsBroken false)
  (Audio|SpawnSoundAttached (Utilities|Select :Index (Math|Random|RandomIntegerinRange 0 1) :Option%200 "/Game/Sounds/Tools/S_Hammer_1.S_Hammer_1" :Option%201 "/Game/Sounds/Tools/S_Hammer_2.S_Hammer_2") (Variables|Default|GetVisualMesh) "None" "0, 0, 0" "0, 0, 0" "KeepRelativeOffset" false 1.0 1.0 0.0 "/Game/Sounds/NewSoundAttenuation.NewSoundAttenuation" 0)
  (for _array_element (Collision|GetOverlappingActors (Variables|Default|GetBox) "/Game/Blueprints/BaseClasses/BP_QuestZOne.BP_QuestZOne_C" :!class /Script/Engine.PrimitiveComponent)
    (bind _asbp_quest_zone (Utilities|Casting|CastToBP_QuestZOne _array_element))
    (Default|UpdateQuest _asbp_quest_zone _self)
    (Development|PrintString "Hello"))
  (Class|CoreQuestSubsystem|UpdateQuest (Subsystems|GetCoreQuestSubsystem) _self))

(fn ConstructionScript
  (Components|StaticMesh|SetStaticMesh (Variables|Default|GetVisualMesh) (Variables|Default|GetBMesh)))

(fn InteractCheck
  (params (Instrument :type Core%20Instrument%20Object%20Object%20Reference))
  (return (and (Utilities|Enum|Equal(Enum) (Variables|/Script/FPS.CoreInstrumentObject_|GetInstrType Instrument) "Hammer") (Variables|Default|GetIsBroken))))

(fn Interactt
  (params (Tool :type Core%20Instrument%20Object%20Object%20Reference))
  (return false))