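; Repairable door that swings open and closed on interaction and hands hammer interactions to its parent class.
; Any non-hammer interaction plays an open or close sound and runs a timeline forward or in reverse to rotate the actor's yaw.
; BeginPlay derives the swing angle and base rotation from the starting yaw and Opened state.
; Finished swings and hammer interactions update the core quest subsystem with different interaction types.
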(event EventBeginPlay
  (bind _returnvalue (Transformation|GetActorRotation))
  (bind (_roll _pitch _yaw) (Math|Rotator|BreakRotator _returnvalue))
  (Variables|Default|SetAngle (- (Variables|Default|GetAngle) (.yaw (Transformation|GetActorRotation))))
  (Variables|Default|SetInitial%20Rot (select (Variables|Default|GetOpened) (Math|Rotator|MakeRotator _roll _pitch (- _yaw (Variables|Default|GetAngle))) _returnvalue)))

(event Collision|EventActorBeginOverlap
  (params (OtherActor :type Actor%20Object%20Reference)))

(event EventTick
  (params (DeltaSeconds :type Float%20%28single-precision%29)))

(event EventInteract
  (params (Instrument :type Core%20Instrument%20Object%20Object%20Reference))
  (bind _initial_rot (Variables|Default|GetInitial%20Rot))
  (if (not (Utilities|ClassIsChildOf (Utilities|GetClass Instrument) "/Game/Blueprints/BaseClasses/InstrumentObjects/BP_BaseHammerObject.BP_BaseHammerObject_C"))
    (Audio|SpawnSoundAttached (select (Variables|Default|GetOpened) "/Game/Sounds/Object/S_Door_Close.S_Door_Close" "/Game/Sounds/Object/S_Door_Open.S_Door_Open") (Variables|Default|GetVisualMesh) "None" "0, 0,140.000000" "0, 0, 0" "KeepRelativeOffset" false 1.0 1.0 0.0 "/Game/Sounds/NewSoundAttenuation.NewSoundAttenuation" 0)
    (if (not (Variables|Default|GetOpened))
      (bind (_direction _rotation) (Timeline|Timeline_0 Play)
        (:Update
          (Transformation|SetActorRotation (Math|Rotator|MakeRotator (.roll _initial_rot) (.pitch _initial_rot) (+ (.yaw _initial_rot) (* _rotation (Variables|Default|GetAngle)))))
          (Variables|Default|SetOpened (Utilities|Enum|Equal(Enum) _direction "Forward")))
        (:Finished
          (Class|CoreQuestSubsystem|UpdateQuest (Subsystems|GetCoreQuestSubsystem) self)))
      (else
        (Timeline|Timeline_0 Reverse)))
    (else
      (|CallParentFunction Instrument)
      (Class|CoreQuestSubsystem|UpdateQuest (Subsystems|GetCoreQuestSubsystem) self 1))))

(fn ConstructionScript)