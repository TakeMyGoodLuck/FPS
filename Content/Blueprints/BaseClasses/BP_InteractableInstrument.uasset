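; Base interactable instrument actor that the player picks up, available only when the core quest subsystem's check on it passes.
; Outline toggles custom-depth highlighting and the interact hint through the game instance, and the hint is hidden on destruction.
; Interacting creates the instrument through the player's ACInstrument component, destroys the actor, then updates the quest.
; InteractCheck and Interactt are stubs returning false.
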(event EventBeginPlay)

(event Collision|EventActorBeginOverlap
  (params (OtherActor :type Actor%20Object%20Reference)))

(event EventTick
  (params (DeltaSeconds :type Float%20%28single-precision%29)))

(event EventOutline
  (params (Start :type Boolean) (Tool :type Core%20Instrument%20Object%20Object%20Reference))
  (bind _result (Class|CoreQuestSubsystem|CheckQuestActor (Subsystems|GetCoreQuestSubsystem) self))
  (if _result
    (Rendering|SetRenderCustomDepth (Variables|Default|GetVisualMesh) Start)
    (Default|ShowInteractHint (CallFunction|GetGI) (Variables|Default|GetInteractKey) (Variables|Default|GetInteractText) Start)
    (else
      (Default|ShowInteractHint (CallFunction|GetGI) "None" "" false))))

(event EventDestroyed
  (Default|ShowInteractHint (CallFunction|GetGI) (Variables|Default|GetInteractKey) "" false))

(event EventInteracted
  (params (Instrument :type Core%20Instrument%20Object%20Object%20Reference))
  (bind _result (Class|CoreQuestSubsystem|CheckQuestActor (Subsystems|GetCoreQuestSubsystem) self))
  (if _result
    (bind _asbp_test_player (Utilities|Casting|CastToBP_TestPlayer (Game|GetPlayerCharacter 0)))
    (Default|CreateInstrument (Variables|/Game/BP_TestPlayer.BP_TestPlayer_C|GetAC_Instrument _asbp_test_player) (Variables|Default|GetInstrumentObject))
    (Actor|DestroyActor)
    (Class|CoreQuestSubsystem|UpdateQuest (Subsystems|GetCoreQuestSubsystem) self)))

(fn ConstructionScript)

(fn InteractCheck
  (params (Instrument :type Core%20Instrument%20Object%20Object%20Reference))
  (return false))

(fn Interactt
  (params (Tool :type Core%20Instrument%20Object%20Object%20Reference))
  (return false))