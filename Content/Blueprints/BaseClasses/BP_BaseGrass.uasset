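; Base grass actor that grows in stages and can be cut with a scythe, then regrows.
; After a random start delay, a timer scaled by growth speed calls GrowGrass, restarting each step until it returns true.
; Scythes get an outline highlight and can cut grass past state 1, resetting growth.
; InstrumentUsed also resets it, plays a short scythe sound, and updates overlapping quest zones and the core quest subsystem.
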(event Custom|Grow
  (bind _ismax (Class|CoreGrassActor|GrowGrass))
  (if _ismax
    (Utilities|Time|ClearandInvalidateTimerbyHandle (Variables|Default|GetTimer))
    (else
      (Utilities|Time|ClearandInvalidateTimerbyHandle (Variables|Default|GetTimer))
      (CallFunction|SetTimer))))

(event Custom|SetTimer
  (bind _returnvalue (Utilities|Time|SetTimerbyEvent (delegate Custom|Grow) (/ 1e+01 (Class|CoreGrassActor|GetGrthSpd)) true))
  (Variables|Default|SetTimer _returnvalue))

(event EventBeginPlay
  (Utilities|FlowControl|Delay (Math|Random|RandomFloatinRange 0.0 7.0))
  (CallFunction|SetTimer))

(event Collision|EventActorBeginOverlap
  (params (OtherActor :type Actor%20Object%20Reference)))

(event EventTick
  (params (DeltaSeconds :type Float%20%28single-precision%29)))

(event EventOutline
  (params (Start :type Boolean) (Tool :type Core%20Instrument%20Object%20Object%20Reference))
  (bind _visualmesh (Variables|Default|GetVisualMesh))
  (if (Utilities|ClassIsChildOf (Utilities|GetClass Tool) "/Game/Blueprints/BaseClasses/InstrumentObjects/BP_BaseScytheObject.BP_BaseScytheObject_C")
    (Rendering|SetRenderCustomDepth _visualmesh Start)
    (else
      (Rendering|SetRenderCustomDepth _visualmesh false))))

(event EventOnGrassGrowed)

(event EventInstrumentUsed
  (params (Instrument :type Core%20Instrument%20Object%20Object%20Reference))
  (Class|CoreGrassActor|Reset)
  (CallFunction|SetTimer)
  (bind _returnvalue (Audio|SpawnSoundAttached "/Game/Sounds/Tools/S_Scythe.S_Scythe" (Variables|Default|GetVisualMesh) "None" "0, 0, 0" "0, 0, 0" "KeepRelativeOffset" false 1.0 1.0 0.0 "/Game/Sounds/NewSoundAttenuation.NewSoundAttenuation" 0))
  (Audio|Components|Audio|StopDelayed _returnvalue 0.4)
  (for _array_element (Collision|GetOverlappingActors (Variables|Default|GetBox) "/Game/Blueprints/BaseClasses/BP_QuestZOne.BP_QuestZOne_C" :!class /Script/Engine.PrimitiveComponent)
    (bind _asbp_quest_zone (Utilities|Casting|CastToBP_QuestZOne _array_element))
    (Default|UpdateQuest _asbp_quest_zone self))
  (Class|CoreQuestSubsystem|UpdateQuest (Subsystems|GetCoreQuestSubsystem) self))

(fn ConstructionScript)

(fn InteractCheck
  (params (Instrument :type Core%20Instrument%20Object%20Object%20Reference))
  (return (and (Utilities|Enum|Equal(Enum) (Variables|/Script/FPS.CoreInstrumentObject_|GetInstrType Instrument) "Scythe") (> (Class|CoreGrassActor|GetState) 1))))

(fn Interactt
  (params (Tool :type Core%20Instrument%20Object%20Object%20Reference))
  (if (Utilities|ClassIsChildOf (Utilities|GetClass Tool) "/Game/Blueprints/BaseClasses/InstrumentObjects/BP_BaseScytheObject.BP_BaseScytheObject_C")
    (if (> (Class|CoreGrassActor|GetState) 1)
      (bind _asbp_base_tool_object (Utilities|Casting|CastToBP_BaseToolObject Tool))
      (if (Class|CoreToolObject|GetIsPossibletoUse _asbp_base_tool_object)
        (Class|CoreGrassActor|Reset)
        (CallFunction|SetTimer)
        (return true)
        (else
          (return false)))
      (else
        (return false)))
    (else
      (return false))))