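; BP_BaseWorldTimer is a base world timer that switches the forest ambience between day and night.
; On BeginPlay it caches the BP_NatureSound actor found in the level.
; Tick watches STime.Hours and sets that actor's audio to the nighttime sound at hour 21 or the daytime sound at hour 7.
; A DoOnce limits the swap to once per switch hour and resets during all other hours.
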(event EventBeginPlay
  (bind _returnvalue (Actor|GetActorOfClass "/Game/Blueprints/BP_NatureSound.BP_NatureSound_C"))
  (Variables|Default|SetNewVar_0 _returnvalue))

(event Collision|EventActorBeginOverlap
  (params (OtherActor :type Actor%20Object%20Reference)))

(event EventTick
  (params (DeltaSeconds :type Float%20%28single-precision%29))
  (bind _stime (Variables|Default|GetSTime))
  (bind _returnvalue (== (.hours _stime) 21))
  (if (or _returnvalue (== (.hours _stime) 7))
    (Utilities|FlowControl|DoOnce false :!label _label
      (:Completed
        (Audio|Components|Audio|SetSound (Variables|/Game/Blueprints/BP_NatureSound.BP_NatureSound_C|GetAudio (Variables|Default|GetNewVar_0)) (Utilities|Select :Index (Math|Integer|SelectInt 0 1 _returnvalue) :Option%200 "/Game/Sounds/World/S_Forest_Nighttime.S_Forest_Nighttime" :Option%201 "/Game/Sounds/World/S_Forest_Daytime.S_Forest_Daytime"))))
    (else
      (goto _label Reset))))

(fn ConstructionScript)