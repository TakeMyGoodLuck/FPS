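; BP_Interactable is a base class for interactable actors tied to the quest system.
; Outline toggles custom depth on the visual mesh and shows or hides a key-and-text hint through the game instance, which is also hidden on destruction.
; Interacted asks the core quest subsystem to validate the actor, then calls OnInteract and updates the quest.
; InteractCheck and Interactt are stubs returning false.
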(event EventBeginPlay)

(event Collision|EventActorBeginOverlap
  (params (OtherActor :type Actor%20Object%20Reference)))

(event EventTick
  (params (DeltaSeconds :type Float%20%28single-precision%29)))

(event EventOutline
  (params (Start :type Boolean) (Tool :type Core%20Instrument%20Object%20Object%20Reference))
  (Rendering|SetRenderCustomDepth (Variables|Default|GetVisualMesh) Start)
  (Default|ShowInteractHint (CallFunction|GetGI) (Variables|Default|GetInteractKey) (Variables|Default|GetInteractText) Start))

(event EventInteracted
  (params (Instrument :type Core%20Instrument%20Object%20Object%20Reference))
  (bind _result (Class|CoreQuestSubsystem|CheckQuestActor (Subsystems|GetCoreQuestSubsystem) self))
  (if _result
    (Default|CallOnInteract)
    (Class|CoreQuestSubsystem|UpdateQuest (Subsystems|GetCoreQuestSubsystem) self)))

(event EventDestroyed
  (Default|ShowInteractHint (CallFunction|GetGI) (Variables|Default|GetInteractKey) "" false))

(fn ConstructionScript)

(fn InteractCheck
  (params (Instrument :type Core%20Instrument%20Object%20Object%20Reference))
  (return false))

(fn Interactt
  (params (Tool :type Core%20Instrument%20Object%20Object%20Reference))
  (return false))