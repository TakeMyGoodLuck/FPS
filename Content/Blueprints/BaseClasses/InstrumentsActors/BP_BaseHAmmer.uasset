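; BP_BaseHAmmer is a base hammer instrument actor that animates its swing when used.
; OnInstrumentUsed scales the timeline play rate by its length over UseSpeed, so UseSpeed acts as the swing duration.
; The timeline drives the VisualMesh relative rotation and location around fixed rest offsets.
; An event track on the same timeline calls a delegate at a keyed moment in the swing.
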(event EventBeginPlay
  (|CallParentFunction) ; This node is disabled and will not be called.\nDrag off pins to build functionality.
)

(event Collision|EventActorBeginOverlap
  (params (OtherActor :type Actor%20Object%20Reference))
  (|CallParentFunction OtherActor) ; This node is disabled and will not be called.\nDrag off pins to build functionality.
)

(event EventTick
  (params (DeltaSeconds :type Float%20%28single-precision%29))
  (|CallParentFunction DeltaSeconds) ; This node is disabled and will not be called.\nDrag off pins to build functionality.
)

(event EventOnInstrumentUsed
  (params (UseSpeed :type Float%20%28single-precision%29))
  (Components|Timeline|SetPlayRate (Variables|Default|GetTimeline_0) (/ (Components|Timeline|GetTimelineLength (Variables|Default|GetTimeline_0)) UseSpeed))
  (bind (_direction _rotation _location) (Timeline|Timeline_0 PlayFromStart)
    (:Update
      (Transformation|SetRelativeRotation (Variables|Default|GetVisualMesh) (Math|Rotator|MakeRotator (.x (+ _rotation (Math|Vector|MakeVector 0.0 3.5e+02 -1e+01))) (.y (+ _rotation (Math|Vector|MakeVector 0.0 3.5e+02 -1e+01))) (.z (+ _rotation (Math|Vector|MakeVector 0.0 3.5e+02 -1e+01)))) false false)
      (Transformation|SetRelativeLocation (Variables|Default|GetVisualMesh) (Math|Vector|MakeVector (.x (+ _location (Math|Vector|MakeVector 0.0 0.0 -23.0))) (.y (+ _location (Math|Vector|MakeVector 0.0 0.0 -23.0))) (.z (+ _location (Math|Vector|MakeVector 0.0 0.0 -23.0)))) false false))
    (:Event
      (Class|BaseInstrumentActor|CallDelegate))))

(fn ConstructionScript
  (|CallParentFunction))