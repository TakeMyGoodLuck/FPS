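; First-person player character for a farming game, carrying seven instruments (gloves, scythe, hoe, rake, hammer, seeds, bucket) created at BeginPlay.
; A short camera trace outlines targets each tick and, on Fire, opens sleep at beds, repairs or fills at workbenches, or uses the current tool, spending stamina and energy.
; Holding QuickAccess shows the instrument picker and locks rotation; ToolSelected swaps the attached tool actor.
; Overlapped grass scales walk speed; K and J feed hunger and thirst.
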(event EventBeginPlay
  (for _index (range 0 6)
    (Default|CreateInstrument (Variables|Default|GetAC_Instrument) (Utilities|Select :Index _index :Option%200 "/Game/Blueprints/GameplayObjects/BP_GlovesObject.BP_GlovesObject_C" :Option%201 "/Game/Blueprints/GameplayObjects/BP_ScytheObject.BP_ScytheObject_C" :Option%202 "/Game/Blueprints/GameplayObjects/BP_HoeObject.BP_HoeObject_C" :Option%203 "/Game/Blueprints/GameplayObjects/BP_RakeObject.BP_RakeObject_C" :Option%204 "/Game/Blueprints/GameplayObjects/BP_HammerObject.BP_HammerObject_C" :Option%205 "/Game/Blueprints/GameplayObjects/BP_SeedsObject.BP_SeedsObject_C" :Option%206 "/Game/Blueprints/GameplayObjects/BP_BucketObject.BP_BucketObject_C")))
  (Variables|Default|SetMax%20Walk%20Speed (Variables|/Script/Engine.CharacterMovementComponent|GetMaxWalkSpeed (Variables|Character|GetCharacterMovement)))
  (CallFunction|ToolSelected (Utilities|Array|Get(acopy) (Default|GetInstruments (Variables|Default|GetAC_Instrument))))
  (bind _returnvalue (UserInterface|CreateWidget "/Game/Blueprints/WidgetBlueprints/PlayerStats/WBP_Time.WBP_Time_C"))
  (UserInterface|Viewport|AddtoViewport _returnvalue 0))

(event Collision|EventActorBeginOverlap
  (params (OtherActor :type Actor%20Object%20Reference)))

(event EventTick
  (params (DeltaSeconds :type Float%20%28single-precision%29))
  (bind _capsulecomponent (Variables|Collision|GetCapsuleComponent))
  (bind _max_walk_speed (Variables|Default|GetMax%20Walk%20Speed))
  (bind _camera (Variables|Default|GetCamera))
  (bind _returnvalue (Transformation|GetWorldLocation _camera))
  (bind _overlappingactors (Collision|GetOverlappingActors _capsulecomponent "/Game/Blueprints/BaseClasses/BP_BaseGrass.BP_BaseGrass_C" :!class /Script/Engine.PrimitiveComponent))
  (bind _output (Utilities|Array|Get(acopy) _overlappingactors))
  (Utilities|FlowControl|Sequence
    (:then_0
      (bind (_outhit _returnvalue_2) (Collision|LineTraceByChannel _returnvalue (+ _returnvalue (* (Math|Vector|GetForwardVector _camera) 2.5e+02)) "TraceTypeQuery3" false 0 "None"))
      (if _returnvalue_2
        (CallFunction|Outline (.HitActor (Collision|BreakHitResult _outhit)))
        (else
          (bind _outlineactor (Variables|Default|GetOutlineActor)
            (:then
              (Class|BPIInteraction|Outline(Message) _outlineactor false (Variables|Default|GetCurrentTool))
              (Variables|Default|SetOutlineActor 0))
            (:else)))))
    (:then_1
      (Utilities|IsValid _output
        (:Is%20Valid
          (bind _asbp_base_grass (Utilities|Casting|CastToBP_BaseGrass _output))
          (Variables|/Script/Engine.CharacterMovementComponent|SetMaxWalkSpeed (Variables|Character|GetCharacterMovement) (Utilities|Select :Index (Class|CoreGrassActor|GetState _asbp_base_grass) :Option%200 _max_walk_speed :Option%201 _max_walk_speed :Option%202 (* _max_walk_speed 0.75) :Option%203 (* _max_walk_speed 0.5)))
          (goto _label Reset))
        (:Is%20Not%20Valid
          (Utilities|FlowControl|DoOnce false :!label _label
            (:Completed
              (Variables|/Script/Engine.CharacterMovementComponent|SetMaxWalkSpeed (Variables|Character|GetCharacterMovement) 6e+02))))))))

(event EventToolSelected
  (params (Tool :type Core%20Instrument%20Object%20Object%20Reference))
  (bind _returnvalue (Game|GetPlayerController 0))
  (bind _currenttool (Variables|Default|GetCurrentTool)
    (:then
      (bind _asbp_base_tool_object (Utilities|Casting|CastToBP_BaseToolObject _currenttool)
        (:then
          (Actor|DestroyActor (Default|GetToolActor _asbp_base_tool_object)))
        (:CastFailed
          _)))
    (:else
      _))
  (bind _output_get (Variables|Default|SetCurrentTool Tool))
  (bind _asbp_base_tool_object_2 (Utilities|Casting|CastToBP_BaseToolObject _output_get)
    (:then
      (bind _returnvalue_2 (Game|SpawnActorfromClass (Variables|/Game/Blueprints/BaseClasses/InstrumentObjects/BP_BaseToolObject.BP_BaseToolObject_C|GetToolClass _asbp_base_tool_object_2) (Variables|/Script/FPS.CoreInstrumentObject_|GetSpwnTransform _output_get) "Undefined" self 0))
      (Default|SetToolActor _asbp_base_tool_object_2 _returnvalue_2)
      (Transformation|AttachComponentToComponent _returnvalue_2 (Variables|Default|GetScene) "None" "KeepRelative" "KeepRelative" "KeepRelative" true))
    (:CastFailed
      _))
  (bind _qa_widget (Variables|Default|GetQA%20Widget)
    (:then
      (Widget|RemovefromParent _qa_widget)
      (Variables|Default|SetQA%20Widget 0)
      (Input|SetInputModeGameOnly _returnvalue)
      (Variables|/Script/Engine.PlayerController|SetbShowMouseCursor _returnvalue false))
    (:else)))

(event Input|ActionEvents|InputActionOpenQA
  (params (Key :type Key%20Structure :default "None")))

(event Input|ActionEvents|InputActionFire
  (params (Key :type Key%20Structure :default "None"))
  (bind _camera (Variables|Default|GetCamera))
  (bind _ac_baseplayerstats (Variables|Default|GetAC_BasePlayerStats))
  (bind _returnvalue (Transformation|GetWorldLocation _camera))
  (:Pressed
    (if (not (Class|UserWidget|IsAnyAnimationPlaying (UserInterface|GetWidget (Variables|Default|GetWidget))))
      (bind (_outhit _returnvalue_2) (Collision|LineTraceByChannel _returnvalue (+ _returnvalue (* (Math|Vector|GetForwardVector _camera) 2.5e+02)) "TraceTypeQuery3" false 0 "None"))
      (if _returnvalue_2
        (Utilities|Casting|CastToBP_BaseBed (.HitActor (Collision|BreakHitResult _outhit))
          (:then
            (bind _returnvalue_3 (UserInterface|CreateWidget "/Game/Blueprints/WidgetBlueprints/WBP_Sleep.WBP_Sleep_C" 0 (Variables|Default|GetAC_BasePlayerStats)))
            (UserInterface|Viewport|AddtoViewport _returnvalue_3 0))
          (:CastFailed
            (Utilities|Casting|CastToCoreWorkbenchA (.HitActor (Collision|BreakHitResult _outhit))
              (:then
                (bind _ascore_tool_object (Utilities|Casting|CastToCoreToolObject (Variables|Default|GetCurrentTool))
                  (:then
                    (Class|CoreToolObject|RepairTool _ascore_tool_object))
                  (:CastFailed
                    (bind _ascore_action_instruments (Utilities|Casting|CastToCoreActionInstruments (Variables|Default|GetCurrentTool)))
                    (Class|CoreActionInstruments|Fill _ascore_action_instruments))))
              (:CastFailed
                (if (and (!= (Class|CorePlayerStats|GetStamina _ac_baseplayerstats) 0.0) (!= (Class|CorePlayerStats|GetEnergy _ac_baseplayerstats) 0.0))
                  (bind _ascore_interactable_actor (Utilities|Casting|CastToCoreInteractableActor (.HitActor (Collision|BreakHitResult _outhit))))
                  (bind (_success _stamina_cost _energy_cost _interact_time _release_time) (Class|CoreInstrumentObject|UseInstrument (Variables|Default|GetCurrentTool) _ascore_interactable_actor))
                  (if _success
                    (Class|BPICrossHair|Interact(Message) (UserInterface|GetWidget (Variables|Default|GetWidget)) _interact_time _release_time)
                    (Class|CorePlayerStats|StaminaReduce (Variables|Default|GetAC_BasePlayerStats) _stamina_cost)
                    (Class|CorePlayerStats|ReduceEnergy (Variables|Default|GetAC_BasePlayerStats) _energy_cost)))))))))))

(event Input|AxisEvents|InputAxisLookUp
  (params (AxisValue :type Float%20%28single-precision%29))
  (if (Variables|Default|GetEnable%20Rotation)
    (Pawn|Input|AddControllerPitchInput AxisValue)))

(event Input|AxisEvents|InputAxisTurn
  (params (AxisValue :type Float%20%28single-precision%29))
  (if (Variables|Default|GetEnable%20Rotation)
    (Pawn|Input|AddControllerYawInput AxisValue)))

(event Input|AxisEvents|InputAxisMoveForward
  (params (AxisValue :type Float%20%28single-precision%29))
  (Pawn|Input|AddMovementInput (Math|Vector|GetForwardVector (Variables|Default|GetCamera)) AxisValue false))

(event Input|AxisEvents|InputAxisMoveRight
  (params (AxisValue :type Float%20%28single-precision%29))
  (Pawn|Input|AddMovementInput (Math|Vector|GetRightVector (Variables|Default|GetCamera)) AxisValue false))

(event Input|AxisEvents|InputAxisQuickAccess
  (params (AxisValue :type Float%20%28single-precision%29))
  (if (== AxisValue 1.0)
    (Variables|Default|GetNewVar_0
      (:then)
      (:else
        (bind _returnvalue (UserInterface|CreateWidget "/Game/Blueprints/WidgetBlueprints/WBP_Instruments.WBP_Instruments_C" 0 (Default|GetInstruments (Variables|Default|GetAC_Instrument)) (Variables|Default|GetCurrentTool)))
        (bind _output_get (Variables|Default|SetNewVar_0 _returnvalue))
        (UserInterface|Viewport|AddtoViewport _output_get 0)
        (Variables|Default|SetEnable%20Rotation false)))
    (else
      (bind _newvar_0 (Variables|Default|GetNewVar_0)
        (:then
          (Widget|RemovefromParent _newvar_0)
          (Variables|Default|SetNewVar_0 0)
          (Variables|Default|SetEnable%20Rotation true))
        (:else)))))

(event Input|KeyboardEvents|K
  (params (Key :type Key%20Structure :default "None"))
  (:Pressed
    (Class|CorePlayerStats|FeedHungry (Variables|Default|GetAC_BasePlayerStats) 1e+01)))

(event Input|KeyboardEvents|J
  (params (Key :type Key%20Structure :default "None"))
  (:Pressed
    (Class|CorePlayerStats|FeedThirst (Variables|Default|GetAC_BasePlayerStats) 25.0)))

(fn ConstructionScript)

(fn Outline
  (params (Actor :type Actor%20Object%20Reference))
  (bind _currenttool (Variables|Default|GetCurrentTool))
  (Variables|Default|GetOutlineActor
    (:then
      (if (== Actor (Variables|Default|GetOutlineActor))
        (Utilities|FlowControl|DoOnce false :!label _label
          (:Completed
            (Class|BPIInteraction|Outline(Message) (Variables|Default|GetOutlineActor) true _currenttool)
            (goto _label_2 Reset)))
        (else
          (Utilities|FlowControl|DoOnce false :!label _label_2
            (:Completed
              (Class|BPIInteraction|Outline(Message) (Variables|Default|GetOutlineActor) false _currenttool)
              (Variables|Default|SetOutlineActor Actor)
              (goto _label Reset))))))
    (:else
      (Variables|Default|SetOutlineActor Actor))))