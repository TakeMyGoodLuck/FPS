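; BP_PlayerController is the player controller that handles input for the pause menu and for closing text and tutorial windows.
; The Return action toggles pause, showing the menu or continuing when its widget is already valid.
; The Close Text action closes the text window if present, otherwise any open tutorial.
; All widget references and open or close calls go through the object returned by GetGI, leaving the controller stateless.
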(event EventBeginPlay)

(event EventTick
  (params (DeltaSeconds :type Float%20%28single-precision%29)))

(event Input|ActionEvents|InputActionReturn
  (params (Key :type Key%20Structure :default "None"))
  (bind _game_instance (CallFunction|GetGI))
  (:Pressed
    (Variables|/Game/Blueprints/BP_GameInstance.BP_GameInstance_C|GetPauseMenuWB _game_instance
      (:then
        (Default|PauseMenuContinue _game_instance))
      (:else
        (Default|ShowPauseMenu _game_instance)))))

(event Input|ActionEvents|InputActionCloseText
  (params (Key :type Key%20Structure :default "None"))
  (bind _game_instance (CallFunction|GetGI))
  (:Pressed
    (Variables|/Game/Blueprints/BP_GameInstance.BP_GameInstance_C|GetText%20Window _game_instance
      (:then
        (Default|CloseText _game_instance))
      (:else
        (Variables|/Game/Blueprints/BP_GameInstance.BP_GameInstance_C|GetTutorialWB _game_instance
          (:then
            (Default|CloseTutorial (CallFunction|GetGI)))
          (:else))))))

(fn ConstructionScript)