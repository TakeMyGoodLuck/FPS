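; Actor component that manages an owner's instruments, tracking the current tool plus separate Tools and Instruments lists.
; SpawnInstrument destroys the current tool, spawns the requested class with an initial health value and makes it current.
; It then removes the first same-class entry from Tools before adding the new actor.
; AddInstrument appends to Instruments, GetTools returns both lists, and the event graph is unused.
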(event EventBeginPlay)

(event EventTick
  (params (DeltaSeconds :type Float%20%28single-precision%29)))

(fn SpawnInstrument
  (params (InstrumentClass :type BP%20Base%20Tool%20Class%20Reference) (InitHealth :type Float%20%28single-precision%29))
  (bind _currenttool (Variables|Default|GetCurrentTool)
    (:then
      (Actor|DestroyActor _currenttool))
    (:else
      _))
  (bind _returnvalue (Game|SpawnActorfromClass InstrumentClass (Utilities|GetClassDefaults InstrumentClass) "AlwaysSpawn" 0 InitHealth 0))
  (Variables|Default|SetCurrentTool _returnvalue)
  (bind _array_element (Utilities|Array|ForEachLoopwithBreak (Variables|Default|GetTools) :!label _label)
    (:LoopBody
      (if (== (Utilities|GetClass _array_element) InstrumentClass)
        (Utilities|Array|RemoveItem (Variables|Default|GetTools) _array_element)
        (goto _label Break)))
    (:Completed
      (Utilities|Array|Add (Variables|Default|GetTools) (Variables|Default|GetCurrentTool))
      (return (Variables|Default|GetCurrentTool)))))

(fn AddInstrument
  (params (NewItem :type BP%20Base%20Tool%20Class%20Reference%20%28by%20ref%29))
  (Utilities|Array|Add (Variables|Default|GetInstruments) NewItem))

(fn GetTools
  (return (Variables|Default|GetTools) (Variables|Default|GetInstruments)))